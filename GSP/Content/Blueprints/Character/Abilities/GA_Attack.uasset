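; GA_Attack is a gameplay ability that fires a projectile from the player character.
; On activation it casts the owner to BP_PlayerCharacter and spawns BP_Projectile at the character's ProjectileSpawnPoint.
; It then applies GE_ReduceHealth to the player's own GSP ability system component and ends, printing debug strings along the way.
; EndAbility is called only when that component is valid.
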(event `self.K2_ActivateAbility`
  (`KismetSystemLibrary.PrintString` "Attack" true true (struct :`R` 1.0 :`G` 0.044643 :`A` 1.0) 1.0)
  (bind _asbp_player_character (cast `/Game/Blueprints/Character/BP_PlayerCharacter` (`.OwnerActor` (break `GameplayAbilityActorInfo` (`self.GetActorInfo`)))))
  (`|SpawnActorFromClass` "/Game/Blueprints/Character/BP_Projectile.BP_Projectile_C" (`SceneComponent.GetSocketTransform` (`GSPCharacter._ProjectileSpawnPoint` _asbp_player_character) "None" "RTS_World") "Undefined" "MultiplyWithRoot" null null)
  (bind _returnvalue (`GSPCharacter.GetGSPAbilitySystemComponent` _asbp_player_character))
  (`/Engine/EditorBlueprintResources/StandardMacros.IsValid` _returnvalue
    (:`Is Valid`
      (`KismetSystemLibrary.PrintString` " yess")
      (`AbilitySystemComponent.BP_ApplyGameplayEffectToSelf` _returnvalue "/Game/Blueprints/Character/Effects/GE_ReduceHealth.GE_ReduceHealth_C" 0.0 (`AbilitySystemComponent.MakeEffectContext` _returnvalue))
      (`self.K2_EndAbility`) ; Ensure you end the Ability
    )
    (:`Is Not Valid`
      (`KismetSystemLibrary.PrintString` "bye"))))