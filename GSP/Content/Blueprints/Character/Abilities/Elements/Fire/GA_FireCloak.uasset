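; GA_FireCloak is the hero's Fire Cloak gameplay ability, which applies GE_FireCloak to the owning BP_HeroCharacter and spawns a BP_FireCloak actor on it.
; The spawned cloak is attached to the hero at zero relative offset, and the cast sound plays at world origin rather than at the hero.
; It commits only the cooldown, then ends immediately, leaving the effect and cloak actor to run independently.
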(event `self.K2_ActivateAbility`
  (bind _owneractor (break `GameplayAbilityActorInfo` (`self.GetActorInfo`)))
  (bind (_returnvalue_location _returnvalue_rotation) (`KismetMathLibrary.BreakTransform` (`Actor.GetTransform` _owneractor)))
  (bind _asbp_hero_character (cast `/Game/Blueprints/Character/BP_HeroCharacter` _owneractor))
  (`AbilitySystemComponent.BP_ApplyGameplayEffectToSelf` (`GSPCharacter.GetAbilitySystemComponent` _asbp_hero_character) "/Game/Blueprints/Character/Abilities/Elements/Fire/GE_FireCloak.GE_FireCloak_C" 0.0 (make `GameplayEffectContextHandle`))
  (bind _returnvalue (`|SpawnActorFromClass` "/Game/Blueprints/Character/Abilities/Elements/Fire/BP_FireCloak.BP_FireCloak_C" (`KismetMathLibrary.MakeTransform` _returnvalue_location _returnvalue_rotation) "AlwaysSpawn" "MultiplyWithRoot" null _asbp_hero_character))
  (`GameplayStatics.PlaySoundAtLocation` "/Game/Assets/Sound/Fire_Cloak__1_.Fire_Cloak__1_" (0.0 0.0 0.0) (struct) 1.0 1.0 0.0 null null null null)
  (`Actor.K2_AttachToActor` _returnvalue _owneractor "None" "KeepRelative" "KeepRelative" "KeepRelative" true)
  (`Actor.K2_SetActorRelativeLocation` _returnvalue (0.0 0.0 0.0) false false)
  (`self.K2_CommitAbilityCooldown` false)
  (`self.K2_EndAbility`))