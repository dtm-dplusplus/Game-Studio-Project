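; Gameplay ability that raises a rock wall on the ground in front of the hero character.
; It offsets from the projectile spawn point and traces straight down on the Visibility channel to find the floor.
; It spawns GSP_RockWall at the hit location with the hero as instigator, aligns its Rock component to the character mesh's rotation, then ends immediately.
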(event `self.K2_ActivateAbility`
  ;[1 1 1] Finds the projectile spawn point of the character, and creates an offset to spawn the wall just in front of the player
  (bind _asbp_hero_character (cast `/Game/Blueprints/Character/BP_HeroCharacter` (`.AvatarActor` (break `GameplayAbilityActorInfo` (`self.GetActorInfo`)))))
  (bind _returnvalue (+ (+ (.location (`SceneComponent.GetSocketTransform` (`GSPCharacter._ProjectileSpawnPoint` _asbp_hero_character) "None" "RTS_World")) (* (`Actor.GetActorForwardVector` _asbp_hero_character) (`KismetMathLibrary.Conv_IntToVector` 200))) (* (`Actor.GetActorRightVector` _asbp_hero_character) (200.0 0.0 0.0))))
  ;[1 1 1] Line trace to find the floor
  (bind _outhit (`KismetSystemLibrary.LineTraceSingle` _returnvalue (- _returnvalue (0.0 0.0 5000.0)) "TraceTypeQuery1"))
  ;[1 1 1] Spawn wall on the floor in front of player. End ability
  (bind _returnvalue_2 (`|SpawnActorFromClass` "/Game/Blueprints/Character/GSP_RockWall.GSP_RockWall_C" (`KismetMathLibrary.MakeTransform` (`.Location` (`GameplayStatics.BreakHitResult` _outhit)) (.rotation (`SceneComponent.GetSocketTransform` (`GSPCharacter._ProjectileSpawnPoint` _asbp_hero_character) "None" "RTS_World")) (.scale (`SceneComponent.GetSocketTransform` (`GSPCharacter._ProjectileSpawnPoint` _asbp_hero_character) "None" "RTS_World"))) "Undefined" "MultiplyWithRoot" null _asbp_hero_character))
  (bind _asbp_hero_character_2 (cast `/Game/Blueprints/Character/BP_HeroCharacter` (`.AvatarActor` (break `GameplayAbilityActorInfo` (`self.GetActorInfo`)))))
  (`SceneComponent.K2_SetWorldRotation` (`/Game/Blueprints/Character/GSP_RockWall.Rock` _returnvalue_2) (`SceneComponent.K2_GetComponentRotation` (`Character.Mesh` _asbp_hero_character_2)) false false)
  (`self.K2_EndAbility`))