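; Player character Blueprint that handles basic movement and mouse look through Enhanced Input.
; IA_Move adds movement relative to control-rotation yaw, and IA_Look_Mouse feeds controller yaw and pitch.
; All other input is left to the abilities system, as noted in the graph.
; A health-changed event prints the new player health as debug text.
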(event `self.ReceiveBeginPlay`)

(event `_OnHealthChanged_Event`
  (params (HealthComponent :type "GSPHealthComponent Object Reference") (OldValue :type "Float (single-precision)") (NewValue :type "Float (single-precision)") (Instigator :type "Actor Object Reference"))
  (`KismetSystemLibrary.PrintString` (`KismetStringLibrary.Concat_StrStr` "Player Health" (`KismetStringLibrary.Conv_DoubleToString` NewValue))))

(event `EnhancedInput|/Game/Blueprints/Input/Actions/IA_Move`
  (params (ActionValue :type "Vector2D Structure") (ElapsedSeconds :type "Float (double-precision)") (TriggeredSeconds :type "Float (double-precision)") (InputAction :type "InputAction Object Reference" :default "/Game/Blueprints/Input/Actions/IA_Move.IA_Move"))
  (bind (_returnvalue_roll _returnvalue_pitch _returnvalue_yaw) (`KismetMathLibrary.BreakRotator` (`self.GetControlRotation`)))
  (bind _returnvalue (`KismetMathLibrary.MakeRotator` 0.0 0.0 _returnvalue_yaw))
  ;[1 1 1] Generic Input Action Handling. The rest of Input are handled by abilities system
  (:`Triggered`
    (`self.AddMovementInput` (`KismetMathLibrary.GetForwardVector` _returnvalue) ActionValue_Y)
    (`self.AddMovementInput` (`KismetMathLibrary.GetRightVector` _returnvalue) ActionValue_X)))

(event `EnhancedInput|/Game/Blueprints/Input/Actions/IA_Look_Mouse`
  (params (ActionValue :type "Vector2D Structure") (ElapsedSeconds :type "Float (double-precision)") (TriggeredSeconds :type "Float (double-precision)") (InputAction :type "InputAction Object Reference" :default "/Game/Blueprints/Input/Actions/IA_Look_Mouse.IA_Look_Mouse"))
  ;[1 1 1] Generic Input Action Handling. The rest of Input are handled by abilities system
  (:`Triggered`
    (`self.AddControllerYawInput` ActionValue_X)
    (`self.AddControllerPitchInput` ActionValue_Y)))

(fn `UserConstructionScript`)