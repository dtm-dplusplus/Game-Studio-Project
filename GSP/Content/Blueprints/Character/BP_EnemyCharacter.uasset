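; BP_EnemyCharacter is an enemy character Blueprint that so far contains only debug scaffolding.
; On BeginPlay it caches the player pawn as PlayerRef and prints a message showing whether that reference is valid.
; A health-changed handler prints the new enemy health, but the node that binds it to the HealthComponent is never executed, so this graph never hooks it up.
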(event `self.ReceiveBeginPlay`
  (bind _output_get (set `self.PlayerRef` (`GameplayStatics.GetPlayerPawn` 0)))
  (`/Engine/EditorBlueprintResources/StandardMacros.IsValid` _output_get
    (:`Is Valid`
      (`KismetSystemLibrary.PrintString` "Hello"))
    (:`Is Not Valid`
      (`KismetSystemLibrary.PrintString` "bye"))))

(event `_OnHealthChanged_Event`
  (params (HealthComponent :type "GSPHealthComponent Object Reference") (OldValue :type "Float (single-precision)") (NewValue :type "Float (single-precision)") (Instigator :type "Actor Object Reference"))
  (`KismetSystemLibrary.PrintString` (`KismetStringLibrary.Concat_StrStr` "Enemy Health" (`KismetStringLibrary.Conv_DoubleToString` NewValue))))

(fn `UserConstructionScript`)