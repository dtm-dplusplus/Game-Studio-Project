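; Behavior tree task for the small robot enemy's self-destruct attack, triggered when the player is very close.
; On AI tick it checks the pawn's distance to the player, failing the task if out of range or the cast fails.
; In range, it zeroes walk speed, prints a detonation warning, then after a short Delay flags the robot as destroyed and succeeds.
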(event `self.ReceiveTickAI`
  (params (OwnerController :type "AIController Object Reference") (ControlledPawn :type "Pawn Object Reference") (DeltaSeconds :type "Float (single-precision)"))
  ;[1 1 1] Small robot detination attack. Similar functionality to the heavy attack; checks for if the player is within distance and then proceeds with the attack.
  (bind _asbp_gsp_enemy_robot_s (cast `/Game/Blueprints/GSP_Enemy/BP_GSP_Enemy_Robot_S` ControlledPawn)
    (:`then`
      (bind _output_get (set `self.As BP GSP Enemy Robot S` _asbp_gsp_enemy_robot_s))
      (if (<= (`KismetMathLibrary.Vector_Distance` (`Actor.K2_GetActorLocation` _asbp_gsp_enemy_robot_s) (`Actor.K2_GetActorLocation` (`GameplayStatics.GetPlayerCharacter` 0))) 10.0)
        (set `CharacterMovementComponent.MaxWalkSpeed` 0.0 (`Character.CharacterMovement` _output_get))
        (`KismetSystemLibrary.PrintString` "DETINATION IN 3 SECONDS")
        (`KismetSystemLibrary.Delay` 3.0)
        (set `/Game/Blueprints/GSP_Enemy/BP_GSP_Enemy_Robot_S.GSP_IsDestroyed` true (`self.As BP GSP Enemy Robot S`))
        (`self.FinishExecute` true)
        (else
          (`self.FinishExecute` false :!label _label))))
    (:`CastFailed`
      (goto _label))))