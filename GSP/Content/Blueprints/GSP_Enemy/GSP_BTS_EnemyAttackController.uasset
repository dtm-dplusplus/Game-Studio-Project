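; Behavior tree service intended to pick an enemy's attack type from its enemy type.
; On each AI tick it casts the controlled pawn to BP_GSP_Enemy and stores the reference, doing nothing further.
; A disconnected chain, which never runs, maps S, M and L types to attack enum values, writes them to the attack-state blackboard key and prints them.
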(event `self.ReceiveTickAI`
  (params (OwnerController :type "AIController Object Reference") (ControlledPawn :type "Pawn Object Reference") (DeltaSeconds :type "Float (single-precision)"))
  ;[1 1 1] Determines what attack the enemy should perform base upon the enemy type.
  (bind _asbp_gsp_enemy (cast `/Game/Blueprints/GSP_Enemy/BP_GSP_Enemy` ControlledPawn))
  (set `self.As BP GSP Enemy` _asbp_gsp_enemy))