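; Behavior tree service that fires the GSP enemy's laser attack.
; On each AI tick, if the blackboard attack type matches the first enum entry, it spawns a GSP_BP_Laser at the enemy's location and rotation.
; It also requires and caches the player character but never aims at it.
; Despite the raycast comment, no trace runs here; a forward end-point calculation is left unused.
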(event `self.ReceiveTickAI`
  (params (OwnerController :type "AIController Object Reference") (ControlledPawn :type "Pawn Object Reference") (DeltaSeconds :type "Float (single-precision)"))
  (bind _as_bp_gsp_enemy (`self.As BP GSP Enemy`))
  ;[1 1 1] Shooting a raycast and if anything blocks it, an effect appears near the location it was blocked.
  (if (== (enumliteral `/Game/Blueprints/GSP_Enemy/GSP_AttackType` "NewEnumerator0") (`BTFunctionLibrary.GetBlackboardValueAsEnum` (`self.GSP_KeyEnemyAttackType`)))
    (`KismetSystemLibrary.PrintString` "LASER ATTACK")
    (bind _asbp_third_person_character (cast `/Game/Blueprints/Character/BP_ThirdPersonCharacter` (`GameplayStatics.GetPlayerCharacter` 0)))
    (set `self.As BP Third Person Character` _asbp_third_person_character)
    (bind _asbp_gsp_enemy (cast `/Game/Blueprints/GSP_Enemy/BP_GSP_Enemy` ControlledPawn))
    (set `self.As BP GSP Enemy` _asbp_gsp_enemy)
    (`KismetSystemLibrary.PrintString` "FIRE")
    (`|SpawnActorFromClass` "/Game/Blueprints/GSP_Enemy/GSP_BP_Laser.GSP_BP_Laser_C" (`KismetMathLibrary.MakeTransform` (`Actor.K2_GetActorLocation` _as_bp_gsp_enemy) (`Actor.K2_GetActorRotation` _as_bp_gsp_enemy)) "AdjustIfPossibleButAlwaysSpawn" "MultiplyWithRoot" null null)
    (`KismetSystemLibrary.PrintString` "LASER SPAWNED")))