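; BP_GSP_Robot_S is the "S" type robot enemy, a child Blueprint that configures and extends inherited enemy behavior.
; On BeginPlay it calls the parent, then sets its health, type tag and speed.
; On actor overlap it runs the parent logic, then destroys itself and prints a "BOOM" debug string if IsExploded is set.
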(event `self.ReceiveBeginPlay`
  (`parent.ReceiveBeginPlay`)
  (set `self.GSP_Health` 50.0)
  (set `self.GSP_EnemyType` "S")
  (set `self.GSP_Speed` 500.0))

(event `self.ReceiveActorBeginOverlap`
  (params (OtherActor :type "Actor Object Reference"))
  (`parent.ReceiveActorBeginOverlap` OtherActor)
  (if (`self.isExploded`)
    (`self.K2_DestroyActor`)
    (`KismetSystemLibrary.PrintString` "BOOM")))

(fn `UserConstructionScript`
  (`parent.UserConstructionScript`))