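; Behavior tree service that sets the enemy's state in the Blackboard from its awareness of the player.
; Each tick it checks AI Perception sight; seeing the player sets the state and target, while losing sight triggers a search.
; Otherwise a nearby player with the crouch flag off counts as heard by distance alone, else the state resets after a delay.
; The last-player-location write is unconnected.
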(event `self.ReceiveTickAI`
  (params (OwnerController :type "AIController Object Reference") (ControlledPawn :type "Pawn Object Reference") (DeltaSeconds :type "Float (single-precision)"))
  ;[1 1 1] Checks to see if the player is visable to the Enemy. The player's visibility then has impact on the enemies actions.
  (`|ExecutionSequence`
    (:`then_0`
      (bind _asbp_third_person_character (cast `/Game/Blueprints/Character/BP_ThirdPersonCharacter` (`GameplayStatics.GetPlayerCharacter` 0)))
      (set `self.As BP Third Person Character` _asbp_third_person_character))
    (:`then_1`
      (bind _asbp_gsp_enemy (cast `/Game/Blueprints/GSP_Enemy/BP_GSP_Enemy` ControlledPawn))
      (bind _output_get (set `self.As BP GSP Enemy` _asbp_gsp_enemy))
      (if (`KismetArrayLibrary.Array_Contains` (`AIPerceptionComponent.GetPerceivedActors` (`/Game/Blueprints/GSP_Enemy/BP_GSP_Enemy._GSP_AIPerception` _output_get) "/Script/AIModule.AISense_Sight") (`GameplayStatics.GetPlayerCharacter` 0))
        (set `self.GSP_HasSeen` true)
        (`BTFunctionLibrary.SetBlackboardValueAsEnum` (`self.GSP_KeyState`) (enumliteral `/Game/Blueprints/GSP_Enemy/GSP_EnemyState` "NewEnumerator1"))
        (`BTFunctionLibrary.SetBlackboardValueAsObject` (`self.GSP_KeyTarget`) (`GameplayStatics.GetPlayerCharacter` 0))
        (elif (`self.GSP_HasSeen`)
          (`self.Search`)
          (set `self.GSP_HasSeen` false)
          (elif (and (<= (`KismetMathLibrary.Vector_Distance` (`Actor.K2_GetActorLocation` (`GameplayStatics.GetPlayerCharacter` 0)) (`Actor.K2_GetActorLocation` (`self.As BP GSP Enemy`))) 500.0) (== (`self.GSP_IsCrouched?`) false))
            (`BTFunctionLibrary.SetBlackboardValueAsEnum` (`self.GSP_KeyState`) (enumliteral `/Game/Blueprints/GSP_Enemy/GSP_EnemyState` "NewEnumerator3"))
            (`KismetSystemLibrary.PrintString` "HEARING-------------------------------")
            (else
              (`KismetSystemLibrary.Delay` 6.0)
              (`BTFunctionLibrary.SetBlackboardValueAsEnum` (`self.GSP_KeyState`) (enumliteral `/Game/Blueprints/GSP_Enemy/GSP_EnemyState` "NewEnumerator0")))))))))

(event `Search`
  ;[1 1 1] Changes the enemy's state to search
  (`BTFunctionLibrary.SetBlackboardValueAsEnum` (`self.GSP_KeyState`) (enumliteral `/Game/Blueprints/GSP_Enemy/GSP_EnemyState` "NewEnumerator2"))
  (`KismetSystemLibrary.PrintString` "SEARCHING"))