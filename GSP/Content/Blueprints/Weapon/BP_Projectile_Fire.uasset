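; Fire projectile that carries a Niagara ray effect and sets struck characters visually aflame.
; On BeginPlay it attaches the ray system to its root component.
; On hit it runs RecieveHit, then AttachFireBurn casts the struck object to GSPCharacter.
; Only when that cast succeeds does it attach a flame system to the character's root and destroy itself.
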(event `self.ReceiveBeginPlay`
  (`NiagaraFunctionLibrary.SpawnSystemAttached` "/Game/Assets/sA_Megapack_v1/sA_Rayvfx/Fx/NiagaraSystems/NS_Ray_1.NS_Ray_1" (`self.RootComponent`) "None" (0.0 0.0 0.0) (struct) "KeepRelativeOffset" true))

(event `self.ReceiveHit`
  (params (MyComp :type "PrimitiveComponent Object Reference") (Other :type "Actor Object Reference") (OtherComp :type "PrimitiveComponent Object Reference") (bSelfMoved :type Boolean) (HitLocation :type "Vector Structure") (HitNormal :type "Vector Structure") (NormalImpulse :type "Vector Structure") (Hit :type "HitResult Structure (by ref)"))
  (`self.RecieveHit` null Other (0.0 0.0 0.0) Hit)
  (`self.AttachFireBurn` Other))

(fn `AttachFireBurn`
  (params (Object :type "Object Object Reference"))
  (bind _asgspcharacter (cast `GSPCharacter` Object))
  (`NiagaraFunctionLibrary.SpawnSystemAttached` "/Game/Assets/sA_Megapack_v1/sA_StylizedAttacksPack/FX/NiagaraSystems/NS_Flame_Single.NS_Flame_Single" (`Actor.RootComponent` _asgspcharacter) "None" (0.0 0.0 0.0) (struct) "KeepRelativeOffset" true)
  (`self.K2_DestroyActor`))

(fn `UserConstructionScript`
  (`parent.UserConstructionScript`))