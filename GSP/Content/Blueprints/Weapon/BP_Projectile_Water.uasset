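; BP_Projectile_Water is a water weapon projectile that knocks back whatever component it hits.
; On BeginPlay it attaches the NS_Ray_4 Niagara system to its root component as the visual effect.
; On hit it passes the hit to RecieveHit, applies a Knockback-scaled impulse along the hitting component's forward vector, then destroys itself.
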(event `self.ReceiveBeginPlay`
  (`NiagaraFunctionLibrary.SpawnSystemAttached` "/Game/Assets/sA_Megapack_v1/sA_Rayvfx/Fx/NiagaraSystems/NS_Ray_4.NS_Ray_4" (`self.RootComponent`) "None" (0.0 0.0 0.0) (struct) "KeepRelativeOffset" true))

(event `self.ReceiveHit`
  (params (MyComp :type "PrimitiveComponent Object Reference") (Other :type "Actor Object Reference") (OtherComp :type "PrimitiveComponent Object Reference") (bSelfMoved :type Boolean) (HitLocation :type "Vector Structure") (HitNormal :type "Vector Structure") (NormalImpulse :type "Vector Structure") (Hit :type "HitResult Structure (by ref)"))
  (`self.RecieveHit` null Other (0.0 0.0 0.0) Hit)
  (`PrimitiveComponent.AddImpulse` OtherComp (* (`SceneComponent.GetForwardVector` MyComp) (`self.Knockback`)) "None" false)
  (`self.K2_DestroyActor`))

(fn `UserConstructionScript`
  (`parent.UserConstructionScript`))