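; BP_Hero_HUD is the player HUD that manages the hero's gameplay UI, small menu and ability wheel.
; On BeginPlay it adds a persistent UI_BaseWidget canvas to the viewport and pushes UI_HUD onto that canvas's widget stack.
; OpenMenu and OpenWheel pop the HUD, push their own widget and switch input to UI-only; only the menu pauses the game.
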(event `self.ReceiveBeginPlay`
  ;[1 1 1] Adds blank UI Canvas to the viewport. Always exists, any UI we want to display gets pushed to its stack
  (bind _output_get (set `self._ControllerRef` (`GameplayStatics.GetPlayerController` 0)))
  (bind _returnvalue (`|CreateWidget` "/Game/Blueprints/UI/UI_BaseWidget.UI_BaseWidget_C" _output_get))
  (bind _output_get_2 (set `self._BaseUI` _returnvalue))
  (set `/Game/Blueprints/UI/UI_BaseWidget._ControllerRef` (`self._ControllerRef`) _output_get_2)
  (`UserWidget.AddToViewport` (`self._BaseUI`) 0)
  (bind _returnvalue_2 (`/Game/Blueprints/UI/UI_BaseWidget.GSP_PushWidget` (`self._BaseUI`) "/Game/Blueprints/UI/UI_HUD.UI_HUD_C"))
  (set `self._HUDUI` _returnvalue_2)
  (set `self._ControllerRef` (`self.GetOwningPlayerController`)))

(event `OpenMenu`
  (bind __baseui (`self._BaseUI`))
  (`/Game/Blueprints/UI/UI_BaseWidget.GSP_PopWidget` __baseui (`self._HUDUI`))
  (bind _returnvalue (`/Game/Blueprints/UI/UI_BaseWidget.GSP_PushWidget` __baseui "/Game/Blueprints/UI/UI_SmallMenu.UI_SmallMenu_C"))
  (bind _asui_small_menu (cast `/Game/Blueprints/UI/UI_SmallMenu` _returnvalue))
  (set `/Game/Blueprints/UI/UI_SmallMenu._Canvas` (`self._BaseUI`) _asui_small_menu)
  (`GameplayStatics.SetGamePaused` true)
  (`WidgetBlueprintLibrary.SetInputMode_UIOnlyEx` (`self._ControllerRef`) null "DoNotLock" true))

(event `OpenWheel`
  (bind __controllerref (`self._ControllerRef`))
  (bind __baseui (`self._BaseUI`))
  (`/Game/Blueprints/UI/UI_BaseWidget.GSP_PopWidget` __baseui (`self._HUDUI`))
  (bind _returnvalue (`/Game/Blueprints/UI/UI_BaseWidget.GSP_PushWidget` __baseui "/Game/Blueprints/UI/UI_AbilityWheel.UI_AbilityWheel_C"))
  (bind _asui_ability_wheel (cast `/Game/Blueprints/UI/UI_AbilityWheel` _returnvalue))
  (bind _output_get (set `self._WheelRef` _asui_ability_wheel))
  (set `/Game/Blueprints/UI/UI_AbilityWheel._ControllerRef` __controllerref _output_get)
  (set `/Game/Blueprints/UI/UI_AbilityWheel._BaseRef` (`self._BaseUI`) _output_get)
  (`WidgetBlueprintLibrary.SetInputMode_UIOnlyEx` __controllerref (`self._WheelRef`)))

(fn `UserConstructionScript`)