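; Behavior tree task meant to pick a location for an enemy to search near the player after losing sight of them.
; Its disconnected node chain would take a random reachable navmesh point within a search radius of the player, write it to a Blackboard key, print it and finish successfully.
; As it stands, the AI tick event is empty, the cast has no target class and none of that logic runs.
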(event `self.ReceiveTickAI`
  (params (OwnerController :type "AIController Object Reference") (ControlledPawn :type "Pawn Object Reference") (DeltaSeconds :type "Float (single-precision)"))
  ;[1 1 1] Determines the radius where the enemy will traverse near after having lost sight of the player
)