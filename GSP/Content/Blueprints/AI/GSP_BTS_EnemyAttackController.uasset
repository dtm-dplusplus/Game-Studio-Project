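; Behavior tree service that chooses an enemy's attack type from its enemy type.
; On each AI tick it casts the controlled pawn to BP_GSP_Enemy and checks for type S, M or L, mapping each to a different attack enum value.
; The result is written to the enemy attack state blackboard key and printed as a debug string.
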(event `self.ReceiveTickAI`
  (params (OwnerController :type "AIController Object Reference") (ControlledPawn :type "Pawn Object Reference") (DeltaSeconds :type "Float (single-precision)"))
  ;[1 1 1] Determines what attack the enemy should perform base upon the enemy type.
  (bind _asbp_gsp_enemy (cast `/Game/Blueprints/AI/BP_GSP_Enemy` ControlledPawn))
  (set `self.As BP GSP Enemy` _asbp_gsp_enemy)
  (`|ExecutionSequence`
    (:`then_0`
      (bind _gsp_enemytype (`/Game/Blueprints/AI/BP_GSP_Enemy.GSP_EnemyType` _asbp_gsp_enemy))
      (if (`KismetStringLibrary.EqualEqual_StrStr` _gsp_enemytype "S")
        (set `self.GSP_EnemyAttackType` "NewEnumerator1")
        (`BTFunctionLibrary.SetBlackboardValueAsEnum` (`self.GSP_KeyEnemyAttackState`) (`self.GSP_EnemyAttackType`) :!label _label)
        (`KismetSystemLibrary.PrintString` (`|GetEnumeratorNameAsString` (`self.GSP_EnemyAttackType`)))))
    (:`then_1`
      (if (`KismetStringLibrary.EqualEqual_StrStr` _gsp_enemytype "M")
        (set `self.GSP_EnemyAttackType` "NewEnumerator0")
        (goto _label)))
    (:`then_2`
      (if (`KismetStringLibrary.EqualEqual_StrStr` _gsp_enemytype "L")
        (set `self.GSP_EnemyAttackType` "NewEnumerator2")
        (goto _label)))))