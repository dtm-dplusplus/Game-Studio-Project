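; A laser actor that destroys any Character it overlaps.
; It caches the player character on BeginPlay, and a cast on overlap filters hits to Characters.
; Each tick it measures its distance to the player and destroys itself once it is too far away, printing debug messages for hits and self-destruction.
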(event `self.ReceiveBeginPlay`
  (set `self.Player Character Ref` (`GameplayStatics.GetPlayerCharacter` 0)))

(event `self.ReceiveActorBeginOverlap`
  (params (OtherActor :type "Actor Object Reference"))
  (bind _ascharacter (cast `Character` OtherActor))
  (`self.K2_DestroyActor` _ascharacter)
  (`KismetSystemLibrary.PrintString` "HIT"))

(event `self.ReceiveTick`
  (params (DeltaSeconds :type "Float (single-precision)"))
  (if (> (`KismetMathLibrary.Vector_Distance` (`self.K2_GetActorLocation`) (`self.K2_GetActorLocation` (`self.Player Character Ref`))) 6000.0)
    (`self.K2_DestroyActor`)
    (`KismetSystemLibrary.PrintString` "DESTROYED")))

(fn `UserConstructionScript`)