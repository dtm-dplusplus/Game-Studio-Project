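; GSP_BTT_EnemyHeavyAttack is a Behavior Tree task stubbing out the heavy attack of the BP_GSP_Robot_L enemy.
; On AI tick it casts the controlled pawn and measures its distance to player 0's character.
; Within close range it prints a debug message and zeroes walk speed, with no damage, animation or speed restore here.
; It finishes successfully whether or not in range, failing only when the cast fails.
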(event `self.ReceiveTickAI`
  (params (OwnerController :type "AIController Object Reference") (ControlledPawn :type "Pawn Object Reference") (DeltaSeconds :type "Float (single-precision)"))
  ;[1 1 1] Heavy Attack Implementation
  (bind _asbp_gsp_robot_l (cast `/Game/Blueprints/AI/BP_GSP_Robot_L` ControlledPawn)
    (:`then`
      (set `self.As BP GSP Robot L` _asbp_gsp_robot_l)
      (if (<= (`KismetMathLibrary.Vector_Distance` (`Actor.K2_GetActorLocation` (`GameplayStatics.GetPlayerCharacter` 0)) (`Actor.K2_GetActorLocation` (`self.As BP GSP Robot L`))) 200.0)
        (`KismetSystemLibrary.PrintString` "ATTACKING")
        (set `CharacterMovementComponent.MaxWalkSpeed` 0.0 (`Character.CharacterMovement` (`self.As BP GSP Robot L`))))
      (`self.FinishExecute` true))
    (:`CastFailed`
      (`self.FinishExecute` false))))