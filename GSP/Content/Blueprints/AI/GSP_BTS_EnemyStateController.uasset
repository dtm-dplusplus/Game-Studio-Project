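; Behavior tree service that picks a GSP enemy's state and writes it to the Blackboard on each AI tick.
; Sight perception of the player sets a seen state and the target, and losing sight switches to search.
; Otherwise, a player within search distance and not crouched triggers a hearing state, using a distance check rather than hearing perception.
; Failing both, a six-second delay precedes the fallback state.
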(event `Search`
  ;[1 1 1] Changes the enemy's state to search
  (`BTFunctionLibrary.SetBlackboardValueAsEnum` (`self._KeyState`) (enumliteral `/Game/Blueprints/AI/GSP_EnemyState` "NewEnumerator2"))
  (`KismetSystemLibrary.PrintString` "SEARCHING"))

(event `self.ReceiveTickAI`
  (params (OwnerController :type "AIController Object Reference") (ControlledPawn :type "Pawn Object Reference") (DeltaSeconds :type "Float (single-precision)"))
  (bind _returnvalue (`GameplayStatics.GetPlayerCharacter` 0))
  ;[1 1 1] Checks to see if the player is visable to the Enemy. The player's visibility then has impact on the enemies actions.
  (`|ExecutionSequence`
    (:`then_0`
      (bind _asbp_gsp_enemy (cast `/Game/Blueprints/AI/BP_GSP_Enemy` ControlledPawn))
      (set `self._EnemyCharacterRef` _asbp_gsp_enemy)
      (`/Engine/EditorBlueprintResources/StandardMacros.IsValid` _returnvalue
        (:`Is Valid`
          (set `self._HeroCharacterRef` _returnvalue))))
    (:`then_1`
      (bind _returnvalue_2 (`self.IsPlayerPercieved`))
      (if _returnvalue_2
        (set `self._HasSeen` true)
        (`BTFunctionLibrary.SetBlackboardValueAsEnum` (`self._KeyState`) (enumliteral `/Game/Blueprints/AI/GSP_EnemyState` "NewEnumerator1"))
        (`BTFunctionLibrary.SetBlackboardValueAsObject` (`self._KeyTarget`) (`self._HeroCharacterRef`))
        (elif (`self._HasSeen`)
          (`self.Search`)
          (set `self._HasSeen` false)
          (elif (and (`self.IsPlayerInRange`) (== (`self._IsHeroCrouched?`) false))
            (`BTFunctionLibrary.SetBlackboardValueAsEnum` (`self._KeyState`) (enumliteral `/Game/Blueprints/AI/GSP_EnemyState` "NewEnumerator3"))
            (`KismetSystemLibrary.PrintString` "HEARING-------------------------------")
            (else
              (`KismetSystemLibrary.Delay` 6.0)
              (`BTFunctionLibrary.SetBlackboardValueAsEnum` (`self._KeyState`) (enumliteral `/Game/Blueprints/AI/GSP_EnemyState` "NewEnumerator0")))))))))

(fn `IsPlayerInRange`
  (returns (ReturnValue :type Boolean))
  (bind __herocharacterref (`self._HeroCharacterRef`))
  (`/Engine/EditorBlueprintResources/StandardMacros.IsValid` __herocharacterref
    (:`Is Valid`
      (return (<= (`KismetMathLibrary.Vector_Distance` (`Actor.K2_GetActorLocation` __herocharacterref) (`Actor.K2_GetActorLocation` (`self._EnemyCharacterRef`))) (`self.SearchDistance?`))))
    (:`Is Not Valid`
      (return false))))

(fn `IsPlayerPercieved`
  (returns (ReturnValue :type Boolean))
  (bind __herocharacterref (`self._HeroCharacterRef`))
  (`/Engine/EditorBlueprintResources/StandardMacros.IsValid` __herocharacterref
    (:`Is Valid`
      (return (`KismetArrayLibrary.Array_Contains` (`AIPerceptionComponent.GetPerceivedActors` (`/Game/Blueprints/AI/BP_GSP_Enemy.AI Perception Comp` (`self._EnemyCharacterRef`)) "/Script/AIModule.AISense_Sight") __herocharacterref)))
    (:`Is Not Valid`
      (return false))))