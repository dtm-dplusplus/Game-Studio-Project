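; BP_GSP_Enemy_Robot_S is the "S" type enemy robot, a child Blueprint that relies on its parent for most behavior.
; BeginPlay calls the parent, then sets its health and type and zeroes its speed.
; Tick calls the parent and polls the destroyed flag, removing the actor after a short Delay once the flag is set.
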(event `self.ReceiveBeginPlay`
  (`parent.ReceiveBeginPlay`)
  (set `self.GSP_Health` 50.0)
  (set `self.GSP_EnemyType` "S")
  (set `self.GSP_Speed` 0.0))

(event `self.ReceiveTick`
  (params (DeltaSeconds :type "Float (single-precision)"))
  (`parent.ReceiveTick` DeltaSeconds)
  (if (`self.GSP_IsDestroyed`)
    (`KismetSystemLibrary.Delay` 3.0)
    (`self.K2_DestroyActor`)))

(fn `UserConstructionScript`
  (`parent.UserConstructionScript`))