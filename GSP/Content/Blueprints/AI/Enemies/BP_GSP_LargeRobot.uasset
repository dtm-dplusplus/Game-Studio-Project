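; BP_GSP_LargeRobot is the large robot enemy, a child Blueprint that sets its own speed and "L" enemy type after the parent's BeginPlay.
; It is weak to water: overlapping a BP_Projectile_Water applies GE_EnemyProjectileDamage to itself through its GSP Ability System Component as extra damage.
; The water hit also prints an "ELEMENTAL" debug string.
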(event `self.ReceiveBeginPlay`
  ;[1 1 1] Assigning the Enemy Specific Values
  (`parent.ReceiveBeginPlay`)
  (set `self.GSP_Speed` 200.0)
  (set `self.GSP_EnemyType` "L"))

(event `self.ReceiveActorBeginOverlap`
  (params (OtherActor :type "Actor Object Reference"))
  (bind _returnvalue (`self.GetGSPAbilitySystemComponent` self))
  ;[1 1 1] Applies Extra damage if hit by a water projectile.
  (cast `/Game/Blueprints/Weapon/BP_Projectile_Water` OtherActor)
  (`KismetSystemLibrary.PrintString` "ELEMENTAL")
  (`AbilitySystemComponent.BP_ApplyGameplayEffectToTarget` :`self` _returnvalue :`GameplayEffectClass` "/Game/Blueprints/Character/Abilities/Enemy_Damages/GE_EnemyProjectileDamage.GE_EnemyProjectileDamage_C" :`Target` _returnvalue))

(fn `UserConstructionScript`
  (`parent.UserConstructionScript`))