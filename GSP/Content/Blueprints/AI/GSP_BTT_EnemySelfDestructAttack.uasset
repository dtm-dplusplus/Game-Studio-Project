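; Behavior tree task that triggers the small enemy robot's self-destruct attack when the player is close.
; On AI tick, it checks the controlled character's distance to the player; in range, it halts movement and prints a detonation warning.
; It flags the first robot found by GetActorOfClass as destroyed, not necessarily the controlled pawn, with no countdown here.
; The task succeeds for any Character regardless of range, otherwise fails.
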(event `self.ReceiveTickAI`
  (params (OwnerController :type "AIController Object Reference") (ControlledPawn :type "Pawn Object Reference") (DeltaSeconds :type "Float (single-precision)"))
  ;[1 1 1] Small robot detination attack. Similar functionality to the heavy attack; checks for if the player is within distance and then proceeds with the attack.
  (bind _ascharacter (cast `Character` ControlledPawn)
    (:`then`
      (`|ExecutionSequence`
        (:`then_0`
          (if (<= (`KismetMathLibrary.Vector_Distance` (`Actor.K2_GetActorLocation` ControlledPawn) (`Actor.K2_GetActorLocation` (`GameplayStatics.GetPlayerCharacter` 0))) 200.0)
            (set `self.GSP_ExecuteAttack` true)
            (set `CharacterMovementComponent.MaxWalkSpeed` 0.0 (`Character.CharacterMovement` _ascharacter))
            (`KismetSystemLibrary.PrintString` "DETINATION IN 3 SECONDS")
            (bind _returnvalue (`GameplayStatics.GetActorOfClass` "/Game/Blueprints/AI/BP_GSP_Enemy_Robot_S.BP_GSP_Enemy_Robot_S_C"))
            (bind _output_get (set `/Game/Blueprints/AI/BP_GSP_Enemy_Robot_S.GSP_IsDestroyed` true _returnvalue))
            (`KismetSystemLibrary.PrintString` (`KismetStringLibrary.Conv_BoolToString` _output_get)))
          (`self.FinishExecute` true))))
    (:`CastFailed`
      (`self.FinishExecute` false))))